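; BP_Enemy is a hazard that patrols back and forth and damages any BP_Sphere it hits.
; Tick moves it along Direction, and a looping timer periodically reverses that vector.
; Each hit sets a debounce timer that then subtracts Damage from the sphere's Health, plays a ping and destroys the sphere at zero.
; On BeginPlay, SetDifficulty reads GameDifficulty from the Game_Vars game instance to scale damage, speed and reversal interval.
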(event `self.ReceiveHit`
  (params (MyComp :type "PrimitiveComponent Object Reference") (Other :type "Actor Object Reference") (OtherComp :type "PrimitiveComponent Object Reference") (bSelfMoved :type Boolean) (HitLocation :type "Vector Structure") (HitNormal :type "Vector Structure") (NormalImpulse :type "Vector Structure") (Hit :type "HitResult Structure (by ref)"))
  ;[1 1 1] Damage Health
  (`KismetSystemLibrary.K2_SetTimerDelegate` (delegate `DecrementHealth`) (`self.TimeDebounceDamage`)))

(event `DecrementHealth`
  ;[1 1 1] Damage Health
  (bind _asbp_sphere (cast `/Game/Blueprints/GameResources/BP_Sphere` (stale `self.ReceiveHit` Other)))
  (set `/Game/Blueprints/GameResources/BP_Sphere.Health` (- (`/Game/Blueprints/GameResources/BP_Sphere.Health` _asbp_sphere) (`self.Damage`)) _asbp_sphere)
  (`GameplayStatics.PlaySoundAtLocation` "/Game/ExternalContent/SuperGrid/TutorialLevel/SoundEffects/ShortPing.ShortPing" (stale `self.ReceiveHit` HitLocation) (struct) 1.0 1.0 0.0 null null null null)
  ;[1 1 1] Kill
  (if (<= (`/Game/Blueprints/GameResources/BP_Sphere.Health` _asbp_sphere) 0.0001)
    (`self.K2_DestroyActor` _asbp_sphere)))

(event `self.ReceiveTick`
  (params (DeltaSeconds :type "Float (single-precision)"))
  ;[1 1 1] Move Enemy
  (`self.K2_AddActorWorldOffset` (* (`KismetMathLibrary.Normal` (`self.Direction`)) (* (`self.Speed`) (`GameplayStatics.GetWorldDeltaSeconds`)))))

(event `self.ReceiveBeginPlay`
  ;[1 1 1] Set Difficulty
  (`self.SetDifficulty`)
  ;[1 1 1] Change Direction
  (`KismetSystemLibrary.K2_SetTimerDelegate` (delegate `ChangeDirection`) (`self.TimeToChange`) true))

(event `ChangeDirection`
  ;[1 1 1] Change Direction
  (set `self.Direction` (* (`self.Direction`) -1.0)))

(fn `SetDifficulty`
  (bind _timetochange (`self.TimeToChange`))
  (bind _asgame_vars (cast `/Game/Blueprints/Game_Vars` (`GameplayStatics.GetGameInstance`)))
  (switch `int` (`/Game/Blueprints/Game_Vars.GameDifficulty` _asgame_vars)
    (:`Default`
      (set `self.Damage` 0.1 :!label _label)
      (set `self.Speed` 200.0)
      (set `self.TimeToChange` (/ _timetochange 1.0)))
    (:`1`
      (goto _label))
    (:`2`
      (set `self.Damage` 0.2)
      (set `self.Speed` 400.0)
      (set `self.TimeToChange` (/ _timetochange 2.0)))
    (:`3`
      (set `self.Damage` 0.25)
      (set `self.Speed` 800.0)
      (set `self.TimeToChange` (/ _timetochange 4.0)))))

(fn `UserConstructionScript`)