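; BP_NextLevel is a next-level marker actor that displays a text title and changes its state once a key is obtained.
; The construction script sets the Title text render to InitialString and applies a color.
; The HasKey event switches the title to FinalString, reapplies a color and destroys the Showcase component.
; It contains no level-loading logic itself.
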(event `Event HasKey`
  (bind _title (`self.Title`))
  (`TextRenderComponent.K2_SetText` _title (`KismetTextLibrary.Conv_StringToText` (`self.FinalString`)))
  (`TextRenderComponent.SetTextRenderColor` _title (make `Color` :`G` 100))
  (`ActorComponent.K2_DestroyComponent` (`self.Showcase`)))

(fn `UserConstructionScript`
  (bind _title (`self.Title`))
  (`TextRenderComponent.K2_SetText` _title (`KismetTextLibrary.Conv_StringToText` (`self.InitialString`)))
  (`TextRenderComponent.SetTextRenderColor` _title (make `Color` :`R` 100)))