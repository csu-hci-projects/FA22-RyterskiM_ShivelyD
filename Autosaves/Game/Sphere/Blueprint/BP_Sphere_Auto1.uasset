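; BP_Sphere is a player-controlled ball that rolls by torque and jumps by impulse on its SMSphere component.
; MoveForwardBack and MoveLeftRight share one torque call that applies axis value times TorqueValue to both X and Y, so the two inputs do not steer separately.
; Jump adds a vertical velocity-change impulse with no ground check.
; The Hit event is an empty stub.
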(event `InputAxis|MoveForwardBack`
  (params (AxisValue :type "Float (single-precision)"))
  ;[1 1 1] Move XY
  (`PrimitiveComponent.AddTorqueInDegrees` (`self.SM_Sphere`) (`KismetMathLibrary.MakeVector` (* (`self.TorqueValue`) (stale `InputAxis|MoveLeftRight` AxisValue)) (* AxisValue (`self.TorqueValue`))) "None" true :!label _label))

(event `InputAxis|MoveLeftRight`
  (params (AxisValue :type "Float (single-precision)"))
  ;[1 1 1] Move XY
  (goto _label))

(event `InputAction|Jump`
  (params (Key :type "Key Structure"))
  (:`Pressed`
    (`PrimitiveComponent.AddImpulse` (`self.SM_Sphere`) (`KismetMathLibrary.MakeVector` 0.0 0.0 (`self.Impulse`)) "None" true)))

(event `self.ReceiveHit`
  (params (MyComp :type "PrimitiveComponent Object Reference") (Other :type "Actor Object Reference") (OtherComp :type "PrimitiveComponent Object Reference") (bSelfMoved :type Boolean) (HitLocation :type "Vector Structure") (HitNormal :type "Vector Structure") (NormalImpulse :type "Vector Structure") (Hit :type "HitResult Structure (by ref)"))
  (if true
    _))

(fn `UserConstructionScript`)